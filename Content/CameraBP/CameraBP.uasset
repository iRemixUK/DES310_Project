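; CameraBP is a player-steered camera actor that rotates with the Turn and LookUp input axes within set angular limits.
; Turn adds yaw in world space and LookUp adds pitch in local space, both scaled by RotationSpeed.
; After each rotation, an out-of-range angle snaps to the nearest min or max limit via SetActorRotation, which also zeroes roll.
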(event `self.ReceiveTick`
  (params (DeltaSeconds :type "Float (single-precision)")))

(event `InputAxis|Turn`
  (params (AxisValue :type "Float (single-precision)"))
  (bind (_returnvalue_roll _returnvalue_pitch _returnvalue_yaw) (`KismetMathLibrary.BreakRotator` (`self.K2_GetActorRotation`)))
  (bind _z_limit_min (`self.Z limit min`))
  (bind _z_limit_max (`self.Z limit max`))
  (bind _returnvalue (< _returnvalue_yaw _z_limit_min))
  (`self.K2_AddActorWorldRotation` (`KismetMathLibrary.MakeRotator` 0.0 0.0 (* AxisValue (`self.RotationSpeed`))))
  (if (or _returnvalue (> _returnvalue_yaw _z_limit_max))
    (`self.K2_SetActorRotation` (`KismetMathLibrary.MakeRotator` 0.0 _returnvalue_pitch (`KismetMathLibrary.SelectFloat` _z_limit_min _z_limit_max _returnvalue)))))

(event `InputAxis|LookUp`
  (params (AxisValue :type "Float (single-precision)"))
  (bind (_returnvalue_roll _returnvalue_pitch _returnvalue_yaw) (`KismetMathLibrary.BreakRotator` (`self.K2_GetActorRotation`)))
  (bind _y_limit_min (`self.Y limit min`))
  (bind _y_limit_max (`self.Y limit max`))
  (bind _returnvalue (< _returnvalue_pitch _y_limit_min))
  (`self.K2_AddActorLocalRotation` (`KismetMathLibrary.MakeRotator` 0.0 (* AxisValue (`self.RotationSpeed`))))
  (if (or _returnvalue (> _returnvalue_pitch _y_limit_max))
    (`self.K2_SetActorRotation` (`KismetMathLibrary.MakeRotator` 0.0 (`KismetMathLibrary.SelectFloat` _y_limit_min _y_limit_max _returnvalue) _returnvalue_yaw))))

(fn `UserConstructionScript`)