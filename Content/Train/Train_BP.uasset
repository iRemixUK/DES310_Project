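; Train Blueprint that moves its mesh along the active path's spline from BeginPlay until it reaches the end.
; A Start timeline sets Speed on each update and enters a short Delay loop that adds Speed to Distance.
; MoveAlong places the mesh at that spline distance in world space, changing location only.
; Movement steps per execution without delta-time scaling, and Travel is set but never read here.
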(event `self.ReceiveBeginPlay`
  (bind _distance (`self.Distance`))
  (bind _spline (`/Game/Train/Path.Spline` (`self.ActivePath`)))
  (bind (_direction _start) (`Timeline|Start` :!via `PlayFromStart`)
    (:`Update`
      (set `self.Speed` _start)
      (set `self.Travel` true)
      (if (< _distance (`SplineComponent.GetSplineLength` _spline)) :!label _label
        (`self.MoveAlong` _spline _distance)
        (set `self.Distance` (+ (`self.Distance`) (`self.Speed`)))
        (`KismetSystemLibrary.Delay` 0.001)
        (goto _label)))))

(fn `MoveAlong`
  (params (Path :type "SplineComponent Object Reference") (Distance :type "Float (double-precision)"))
  (`SceneComponent.K2_SetWorldLocation` (`self.TrainMesh`) (`SplineComponent.GetLocationAtDistanceAlongSpline` Path Distance "World") false false))

(fn `UserConstructionScript`)